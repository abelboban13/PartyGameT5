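; BP_PartyGameMode is a party game mode that runs turn-based rounds of die rolls for every BP_Character in the level.
; BeginPlay stores the characters as the turn order, which each round copies into a queue.
; The front character rolls and its OnTurnEnded event advances the queue.
; An empty queue decrements Rounds and restarts after a delay marked for a future minigame, with no end-of-game check.
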(event `self.ReceiveBeginPlay`
  (bind _outactors (`GameplayStatics.GetAllActorsOfClass` "/Game/ProjectFiles/Blueprints/Character/BP_Character.BP_Character_C"))
  (set `self.TurnOrder` _outactors)
  (`self.InitiateRound`))

(event `InitiateRound`
  (set `self.RoundOrder` (`self.TurnOrder`))
  (`self.StartTurn`))

(event `StartTurn`
  (bind _output (`|GetArrayItem` (`self.RoundOrder`)))
  (`/Game/ProjectFiles/Blueprints/Character/BP_Character.RollDie` _output)
  (add `/Game/ProjectFiles/Blueprints/Character/BP_Character.OnTurnEnded` _output (delegate `NextTurn`)))

(event `NextTurn`
  (`KismetArrayLibrary.Array_Remove` (`self.RoundOrder`))
  (if (`KismetArrayLibrary.Array_IsEmpty` (`self.RoundOrder`))
    (`self.EndRound`)
    (else
      (`self.StartTurn`))))

(event `EndRound`
  (`/Engine/EditorBlueprintResources/StandardMacros.DecrementInt` (`self.Rounds`)
    (:`  `
      ;[1 1 1] Where minigame Starts
      (`KismetSystemLibrary.Delay` 3.0)
      (`self.InitiateRound`))))

(fn `UserConstructionScript`)