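; Board-game player character that rolls a die, walks along linked spaces and resolves the space it lands on.
; RollDie blends the camera to the character and runs the W_Roll widget, whose stop event starts a recursive AI MoveTo countdown through each first NextSpace link.
; At turn end the space type adjusts coins, trades coins for mangoes (or grants coins if short), or flags a skipped turn, then turn-ended and coin events fire.
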(event `self.ReceiveBeginPlay`
  (bind _asw_roll (cast `/Game/ProjectFiles/Blueprints/Widgets/W_Roll` (`WidgetComponent.GetWidget` (`self.Widget`))))
  (set `self.As W Roll` _asw_roll))

(event `MoveToSpace`
  (params (CurrentSpace :type "/Game/ProjectFiles/Blueprints/Board/BP_BoardSpace Object Reference"))
  (bind _output (`|GetArrayItem` (`/Game/ProjectFiles/Blueprints/Board/BP_BoardSpace.NextSpace` CurrentSpace)))
  ;[1 1 1] Move To Space
  (set `self.CurrentSpace` _output)
  (`|AIMoveTo` self (0.0 0.0 0.0) _output
    (:`OnSuccess`
      (bind _result (`/Engine/EditorBlueprintResources/StandardMacros.DecrementInt` (`self.MovesRemaining`))
        (:`  `
          (`TextBlock.SetText` (`/Game/ProjectFiles/Blueprints/Widgets/W_Roll.TXT_Number` (`self.As W Roll`)) (`KismetTextLibrary.Conv_IntToText` _result))
          (if (> _result 0)
            (`self.MoveToSpace` (`self.CurrentSpace`))
            (else
              (`self.TurnEnded`))))))))

(event `TurnEnded`
  (bind _as_w_roll (`self.As W Roll`))
  ;[1 1 1] End Turn
  (clear `/Game/ProjectFiles/Blueprints/Widgets/W_Roll.OnRollStopped` _as_w_roll)
  (`Widget.SetVisibility` _as_w_roll "Hidden")
  (`KismetSystemLibrary.Delay` 3.0)
  (`|ExecutionSequence`
    (:`then_0`
      (switch `/Game/ProjectFiles/Blueprints/Board/E_SpaceType` (`/Game/ProjectFiles/Blueprints/Board/BP_BoardSpace.SpaceType` (`self.CurrentSpace`))
        (:`NewEnumerator0`
          (`self.AddCoins` 3))
        (:`NewEnumerator1`
          (`self.AddCoins` -3))
        (:`NewEnumerator3`
          (`self.AddMangoes` 1))
        (:`NewEnumerator4`
          (`self.Skip Turn`))))
    (:`then_1`
      (`self.OnTurnEnded`)
      (`self.OnCoinCollected`))))

(event `RollDie`
  (bind _as_w_roll (`self.As W Roll`))
  ;[1 1 1] Roll Die
  (if (`self.isSkipped?`)
    (`KismetSystemLibrary.Delay` 2.0)
    (`self.OnTurnEnded`)
    (set `self.isSkipped?` false)
    (else
      (`PlayerController.SetViewTargetWithBlend` (`GameplayStatics.GetPlayerController` 0) self 1.0 "VTBlend_Linear" 0.0 false)
      (`/Game/ProjectFiles/Blueprints/Widgets/W_Roll.StartRoll` _as_w_roll)
      (add `/Game/ProjectFiles/Blueprints/Widgets/W_Roll.OnRollStopped` _as_w_roll (delegate `RollStopped`))
      (`Widget.SetVisibility` _as_w_roll "Visible"))))

(event `RollStopped`
  (params (Number :type Integer))
  ;[1 1 1] Roll Die
  (set `self.MovesRemaining` Number)
  (`self.MoveToSpace` (`self.CurrentSpace`)))

(fn `AddCoins`
  (params (Number :type Integer :default 0))
  (set `self.Coins` (+ (`self.Coins`) Number)))

(fn `AddMangoes`
  (params (Number :type Integer))
  (if (>= (`self.Coins`) 40)
    (set `self.Mangoes` (+ Number (`self.Mangoes`)))
    (set `self.Coins` (- (`self.Coins`) 40))
    (else
      (set `self.Coins` (+ (`self.Coins`) 40)))))

(fn `Skip Turn`
  (set `self.isSkipped?` true))

(fn `UserConstructionScript`)