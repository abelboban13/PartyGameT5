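; BP_Enemy runs a red light, green light game, ragdolling the player character if it moves during a freeze.
; A looping BeginPlay sequence alternates IsFreeze on random timers, turning its light red or green.
; Parallel warning events roll each duration and print FREEZE one second early, and UNFREEZE as the freeze ends.
; While frozen, Tick checks player velocity against a small threshold and enables mesh physics simulation when exceeded.
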(event `self.ReceiveBeginPlay`
  ;[1 1 1] Main Loop
  (`self.FreezeWarning` :!label _label)
  (`KismetSystemLibrary.Delay` (`self.FreezeTimer`))
  (set `self.IsFreeze?` true)
  (`LightComponent.SetLightColor` (`self.Light`) (struct :`R` 1.0 :`A` 1.0) true)
  (`self.UnfreezeWarning`)
  (`KismetSystemLibrary.Delay` (`self.UnfreezeTimer`))
  (set `self.IsFreeze?` false)
  (`LightComponent.SetLightColor` (`self.Light`) (struct :`G` 1.0 :`B` 0.103821 :`A` 1.0) true)
  (goto _label))

(event `self.ReceiveTick`
  (params (DeltaSeconds :type "Float (single-precision)"))
  ;[1 1 1] Check Player Speed
  (if (`self.IsFreeze?`)
    (bind _asbp_third_person_character (cast `/Game/ThirdPerson/Blueprints/BP_ThirdPersonCharacter` (`GameplayStatics.GetPlayerCharacter` 0)))
    (if (>= (`KismetMathLibrary.VSize` (`self.GetVelocity` _asbp_third_person_character)) 20.0)
      (`PrimitiveComponent.SetSimulatePhysics` (`Character.Mesh` _asbp_third_person_character) true))))

(event `FreezeWarning`
  (bind _returnvalue (- (`self.FreezeTimer`) 1.0))
  ;[1 1 1] Freeze Warning
  (set `self.FreezeTimer` (`KismetMathLibrary.Conv_IntToDouble` (`KismetMathLibrary.RandomIntegerInRange` 3 6)))
  (set `self.StopPrep` _returnvalue)
  (`KismetSystemLibrary.Delay` _returnvalue)
  (`KismetSystemLibrary.PrintString` "FREEZE" true true (struct :`R` 1.0 :`A` 1.0)))

(event `UnfreezeWarning`
  ;[1 1 1] Unfreeze Warning
  (bind _output_get (set `self.UnfreezeTimer` (`KismetMathLibrary.Conv_IntToDouble` (`KismetMathLibrary.RandomIntegerInRange` 3 6))))
  (`KismetSystemLibrary.Delay` _output_get)
  (`KismetSystemLibrary.PrintString` "UNFREEZE" true true (struct :`G` 1.0 :`B` 0.103821 :`A` 1.0)))

(fn `UserConstructionScript`)